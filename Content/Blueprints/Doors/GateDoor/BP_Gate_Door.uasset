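; Gate door Blueprint that slides its door upward and plays a placeholder explosion sound, with movement meant to be started by BP_GateTrigger.
; StartMovingDoor fires the sound function, then plays a timeline that lerps the door's relative Z up to a fixed height.
; Tick flags when that height is reached, so each timeline update can stop further movement.
; DoOnce gates, one reset after a retriggerable delay, throttle the debug messages.
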(event Custom|PreventRepeatOnLocationSet
  ;[1 0 0.1805] Prevention of Multiple Execution of Timelines (End Custom Event)
  (if (Variables|Booleans|GetbHasLocationValueBeenReached?)
    (Utilities|FlowControl|Sequence
      (:then_0
        (Utilities|FlowControl|DoOnce false :!label _label ; Preventing Multiple Prints all at once
          (:Completed
            (Development|PrintString "GATEDOOR: An attempt to move GateDoor has failed because the Location Z Value is Greater than or Equal to 100. " true true "(R=1.000000,G=0.000000,B=0.026767,A=1.000000)")
            ;[0.8854 0.3695 1] Using Timeline with Lerp to set a New Location Z for Gate Door to move UP
            (bind _alpha (Timeline|MoveUpTimeline Stop)
              (:Update
                (bind _output_get (Variables|Locations|SetNew%20Location%20Z%20%28Lerp%29%20%28Up%29 (Math|Float|Lerp 0.0 1e+02 _alpha)))
                (Transformation|SetRelativeLocation (Variables|Default|GetGateDoor) (Math|Vector|MakeVector 0.0 0.0 _output_get) false false)
                ;;[1 0 0] Preventing Repeat Execution
                (CallFunction|PreventRepeatonLocationSet))))))
      (:then_1
        (Utilities|FlowControl|RetriggerableDelay 2.0) ; To allow reprint
        (goto _label Reset)))
    (else
      (Utilities|FlowControl|DoOnce false
        (:Completed
          (Variables|Default|SetbHasGateDoorMoved? true)
          (Development|PrintString "GateDoor: Gate is still moving. Please Wait" true true "(R=1.000000,G=0.837037,B=0.000000,A=1.000000)") ; I only intend this to print once. Unless there are multiple instances of this Blueprint
        )))))

(event Custom|StartMovingDoor
  ;[0.8854 0.3695 1] Using Timeline with Lerp to set a New Location Z for Gate Door to move UP
  (Utilities|FlowControl|Sequence
    (:then_0
      (Utilities|CallSoundEffect(GateDoor)))
    (:then_1
      (bind _alpha (Timeline|MoveUpTimeline Play)
        (:Update
          (bind _output_get (Variables|Locations|SetNew%20Location%20Z%20%28Lerp%29%20%28Up%29 (Math|Float|Lerp 0.0 1e+02 _alpha)))
          (Transformation|SetRelativeLocation (Variables|Default|GetGateDoor) (Math|Vector|MakeVector 0.0 0.0 _output_get) false false)
          ;;[1 0 0] Preventing Repeat Execution
          (CallFunction|PreventRepeatonLocationSet))))))

(event EventTick
  (params (DeltaSeconds :type Float%20%28single-precision%29))
  ;[1 0 0] Condition Checks
  (Variables|Booleans|SetbHasLocationValueBeenReached? (>= (Variables|Locations|GetNew%20Location%20Z%20%28Lerp%29%20%28Up%29) 1e+02)) ; This is used for the "PreventRepeatOnLocationSet" Event
)

(fn ConstructionScript)