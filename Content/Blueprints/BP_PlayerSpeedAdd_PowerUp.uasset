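; BP_PlayerSpeedAdd_PowerUp is a power-up that permanently raises the player's walk speed when touched.
; On BeginPlay it caches the player pawn as BP_FirstPersonCharacter.
; A box overlap by an actor tagged Player passes a DoOnce, adds a fixed bonus to the cached character's MaxWalkSpeed and prints debug messages.
; The pickup fires only once but is not destroyed or hidden afterward.
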(event OnComponentBeginOverlap(Box)
  (params (OverlappedComponent :type Primitive%20Component%20Object%20Reference) (OtherActor :type Actor%20Object%20Reference) (OtherComp :type Primitive%20Component%20Object%20Reference) (OtherBodyIndex :type Integer) (bFromSweep :type Boolean) (SweepResult :type Hit%20Result%20Structure%20%28by%20ref%29))
  (if (Actor|ActorHasTag OtherActor "Player")
    (Utilities|FlowControl|DoOnce false
      (:Completed
        (bind _output_get (Variables|/Game/Blueprints/PlayerBlueprints/BP_FirstPersonCharacter.BP_FirstPersonCharacter_C|SetMax%20Walk%20Speed (Variables|Default|GetAs%20BP%20First%20Person%20Character) (+ (Variables|/Game/Blueprints/PlayerBlueprints/BP_FirstPersonCharacter.BP_FirstPersonCharacter_C|GetMax%20Walk%20Speed (Variables|Default|GetAs%20BP%20First%20Person%20Character)) 15.0)))
        (Utilities|FlowControl|Sequence
          (:then_0
            (Development|PrintString "PLAYER: Walk Speed should be increased by f15.0"))
          (:then_1
            (Development|PrintString (Utilities|String|ToString(Float) _output_get))))))))

(event EventBeginPlay
  (bind _asbp_first_person_character (Utilities|Casting|CastToBP_FirstPersonCharacter (Game|Player|GetPlayerPawn 0)))
  (Variables|Default|SetAs%20BP%20First%20Person%20Character _asbp_first_person_character))

(fn ConstructionScript)