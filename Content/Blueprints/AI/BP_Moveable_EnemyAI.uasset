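; Moveable enemy AI that pursues the player and can be damaged and killed.
; BeginPlay and pawn sensing start RandomRoam if EnableAI, toggled by keys 5 and 6, is set.
; It reissues AIMoveTo every two seconds with both a random reachable point and the player as target actor, without rechecking the flag.
; AnyDamage reduces health; death enables mesh physics, plays a sound and destroys the actor after a delay.
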(event OnSeePawn(PawnSensing)
  (params (Pawn :type Pawn%20Object%20Reference))
  (CallFunction|RandomRoam))

(event Custom|RandomRoam
  (if (Variables|Default|GetbEnableAI?)
    (bind _movementresult (AI|AIMoveTo self (.RandomLocation (AI|Navigation|GetRandomReachablePointinRadius (Transformation|GetActorLocation) 2e+03 0 0)) (Game|GetPlayerCharacter 0) 5.0 false :!label _label)
      (:then
        (Utilities|FlowControl|Delay 2.0)
        (goto _label))
      (:OnSuccess
        (Development|PrintString (Utilities|String|EnumtoString _movementresult))
        (Development|PrintString "SUCCESS: AI is moving towards player"))
      (:OnFail
        (Development|PrintString "FAIL: AI can see player but can't follow " true true "(R=0.000000,G=0.660000,B=1.000000,A=1.000000)" 0.0002)))))

(event Custom|DamageAI
  (bind _returnvalue (Game|Damage|ApplyDamage self 1e+01 0 0))
  (Development|PrintString (Utilities|String|ToString(Float) _returnvalue)))

(event Game|Damage|EventAnyDamage
  (params (Damage :type Float%20%28single-precision%29) (DamageType :type Damage%20Type%20Object%20Reference) (InstigatedBy :type Controller%20Object%20Reference) (DamageCauser :type Actor%20Object%20Reference))
  ;[0 1 0.2355] AI Health System
  (Variables|Default|SetAIHealth (- (Variables|Default|GetAIHealth) Damage))
  (if (<= (Variables|Default|GetAIHealth) 0.0)
    (Utilities|FlowControl|DoOnce false
      (:Completed
        (Development|PrintString "MOVINGAI: AI Eliminated" true true "(R=1.000000,G=0.000000,B=0.000000,A=1.000000)")
        ;[1 0 0.1612] When Health Hits Zero, preform these functions
        (Physics|SetSimulatePhysics (Variables|Default|GetFirstPersonMesh) true)
        (Audio|PlaySoundatLocation "/Engine/VREditor/Sounds/UI/Camera_Shutter.Camera_Shutter" (Transformation|GetActorLocation self) "0, 0, 0" 0.002 1.0 0.0 0 0 0 0) ; Need Appropriate SFX
        (Utilities|FlowControl|Delay 2.0)
        (Actor|DestroyActor)))
    (else
      (Development|PrintString (Utilities|String|ToString(Float) (Variables|Default|GetAIHealth)) true true "(R=0.036493,G=1.000000,B=0.000000,A=1.000000)"))))

(event EventBeginPlay
  (CallFunction|RandomRoam))

(event Input|KeyboardEvents|6
  (params (Key :type Key%20Structure :default "None"))
  (:Pressed
    (Variables|Default|SetbEnableAI? false)))

(event Input|KeyboardEvents|5
  (params (Key :type Key%20Structure :default "None"))
  (:Pressed
    (Variables|Default|SetbEnableAI? true)))

(fn ConstructionScript)