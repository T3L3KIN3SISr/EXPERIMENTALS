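; Game instance that enforces and restores the user's display settings when the game starts.
; On Init, a sequence runs four collapsed graphs against GameUserSettings.
; They turn VSync off, restore the last confirmed fullscreen mode and screen resolution, and re-set the current texture quality.
; The VSync step has no apply call of its own and relies on the later ApplySettings calls.
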(event EventInit
  (Utilities|FlowControl|Sequence
    (:then_0
      (|CollapseGraph))
    (:then_1
      (|CollapseGraph_0))
    (:then_2
      (|CollapseGraph_1))
    (:then_3
      (|CollapseGraph_2))))