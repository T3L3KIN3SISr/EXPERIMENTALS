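; Pickable flashlight actor that the player collects through an Interaction event.
; Interaction notifies the first-person character and a referenced door's intro flashlight event, plays an equip sound, then destroys the actor after a short delay.
; An outline overlay material is applied at BeginPlay and cleared on overlap end, without being reapplied.
; Overlap begin and end also show and hide the interact widget.
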(event EventInteraction
  (bind _asbp_first_person_character (Utilities|Casting|CastToBP_FirstPersonCharacter (Game|Player|GetPlayerPawn 0))
    (:then
      (Default|PickedUpFlashlight? _asbp_first_person_character)
      (Default|INTROFlashlight (Variables|Default|GetDoorReference))
      (Audio|PlaySound2D "/Game/Audio/SW_item-equip-6904.SW_item-equip-6904" 1.0 1.0 0.0 0 0)
      (Utilities|FlowControl|Delay 1.0)
      (Actor|DestroyActor))
    (:CastFailed
      (Development|PrintString "Flashlight: AIN't casting L'ssss"))))

(event EventBeginPlay
  ;[1 1 1] Add Material Overlay when Player is near
  ;;[0.2075 1 0] On
  (Rendering|Material|SetOverlayMaterial (Variables|Default|GetSM_Flashlight) "/Game/Materials/M_OutlineInteract_Inst.M_OutlineInteract_Inst" :!class /Script/Engine.MeshComponent))

(event Collision|EventActorBeginOverlap
  (params (OtherActor :type Actor%20Object%20Reference))
  ;[1 1 1] Add Material Overlay when Player is near
  ;;[0.01982 0 1] Set Widget Visibility
  (Rendering|SetVisibility (Variables|Default|GetInteractWidget) true false))

(event Collision|EventActorEndOverlap
  (params (OtherActor :type Actor%20Object%20Reference))
  ;[1 1 1] Add Material Overlay when Player is near
  ;;[1 0 0] Off
  (Rendering|Material|SetOverlayMaterial (Variables|Default|GetSM_Flashlight) 0 :!class /Script/Engine.MeshComponent)
  ;;[0.01982 0 1] Set Widget Visibility
  (Rendering|SetVisibility (Variables|Default|GetInteractWidget) false false))

(fn ConstructionScript)