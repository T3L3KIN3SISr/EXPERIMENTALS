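; BP_DeathTrigger is an invisible trigger that kills the player on contact and restarts the level.
; When an actor tagged "Player" overlaps its box collision, it casts to BP_FirstPersonCharacter and disables that character's movement.
; It then shows the WB_PlayerDeath widget with a 2D sound, waits for the animation to finish, and reopens the current level by name.
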(event OnComponentBeginOverlap(BoxCollision)
  (params (OverlappedComponent :type Primitive%20Component%20Object%20Reference) (OtherActor :type Actor%20Object%20Reference) (OtherComp :type Primitive%20Component%20Object%20Reference) (OtherBodyIndex :type Integer) (bFromSweep :type Boolean) (SweepResult :type Hit%20Result%20Structure%20%28by%20ref%29))
  ;[1 0.839 0] Check if the "Player" Tag has hit the Collision
  (if (Actor|ActorHasTag OtherActor "Player")
    (bind _asbp_first_person_character (Utilities|Casting|CastToBP_FirstPersonCharacter OtherActor)) ; Casting due to BP already being in Instance
    ;[0.4485 0.3441 1] Disable Movement and Print String
    (Development|PrintString "DeathTrigger : Restarting Instance" true true "(R=0.000000,G=1.000000,B=0.105656,A=1.000000)")
    (Pawn|Components|CharacterMovement|DisableMovement (Variables|/Script/Engine.Character|GetCharacterMovement _asbp_first_person_character)) ; Stop the Player from Moving when they have hit the Death Trigger
    (bind _returnvalue (Game|GetCurrentLevelName true))
    ;[1 0 0.03209] Show Death UI on the Player
    (bind _returnvalue_2 (Game|ConstructObjectfromClass (Variables|/Script/Engine.Character|GetCharacterMovement _asbp_first_person_character) "/Game/UI/PlayerConditions/WB_PlayerDeath.WB_PlayerDeath_C")) ; This will show on Player
    (Audio|PlaySound2D "/Engine/EditorSounds/Notifications/CompileFailed.CompileFailed" 1.0 1.0 0.0 0 0) ; Find Appropriate SFX
    (UserInterface|Viewport|AddtoViewport _returnvalue_2 0)
    (Utilities|FlowControl|Delay 5.0) ; Let the UI Widget finish its Animation
    ;[0.004252 1 0] Reload the Current Level
    (Game|OpenLevel(byName) (Utilities|String|StringToName _returnvalue))))

(fn ConstructionScript)