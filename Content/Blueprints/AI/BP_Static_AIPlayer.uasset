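; Static AI enemy that turns to face and shoot at the first-person player when PawnSensing sees them.
; After a configurable delay it spawns a projectile along its Arrow, later destroying it, and plays a one-time alert sound on first sighting.
; Box hits from tagged actors and the InstaKill event feed AnyDamage, which lowers health.
; At zero health it enables physics, plays a sound and destroys itself after a delay.
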(event OnSeePawn(PawnSensing)
  (params (Pawn :type Pawn%20Object%20Reference))
  ;[1 0.8075 0] Look at the Player when they are near.
  (Utilities|FlowControl|Sequence
    (:then_0
      (Utilities|Casting|CastToBP_FirstPersonCharacter Pawn) ; Get Active Instance
      (Transformation|SetActorRotation (Math|Rotator|MakeRotator 0.0 0.0 (.yaw (Math|Rotator|FindLookatRotation (Transformation|GetActorLocation) (Transformation|GetActorLocation Pawn)))))
      ;[0.6652 0.1511 1] Spawn Bullet towards Player
      (Utilities|FlowControl|Delay (Variables|Delays|GetBulletSpawnDelayWhenSeen))
      (bind _returnvalue (Game|SpawnActorfromClass (Variables|ShootableObject|GetShootObject) (Transformation|GetWorldTransform (Variables|Default|GetArrow)) "Undefined" "MultiplyWithRoot" 0 0))
      (Audio|SpawnSoundatLocation "/Game/Misc/FPWeapon/Audio/FirstPersonTemplateWeaponFire02.FirstPersonTemplateWeaponFire02" (Transformation|GetWorldLocation (Variables|Default|GetStaticMesh)) "0, 0, 0" 0.5 1.0 0.0 0 0)
      ;[0.2205 1 0.09279] Check for Object Validity to prevent Garbage Errors and then Destroy Actor
      (Utilities|FlowControl|Delay 1e+01)
      (Utilities|IsValid _returnvalue
        (:Is%20Valid
          (Actor|DestroyActor _returnvalue))
        (:Is%20Not%20Valid
          (Development|PrintString "Attempted to Delete Object but is not Valid" false true "(R=0.000000,G=0.660000,B=1.000000,A=1.000000)" 1e-05))))
    (:then_1
      (Utilities|FlowControl|DoOnce false
        (:Completed
          (Audio|PlaySound2D "/Engine/VREditor/Sounds/UI/Invalid_Action.Invalid_Action" 1.0 1.0 0.0 0 0))))))

(event OnComponentHit(Box)
  (params (HitComponent :type Primitive%20Component%20Object%20Reference) (OtherActor :type Actor%20Object%20Reference) (OtherComp :type Primitive%20Component%20Object%20Reference) (NormalImpulse :type Vector :default "0, 0, 0") (Hit :type Hit%20Result%20Structure%20%28by%20ref%29))
  ;[1 0.7044 0.1557] Check if "Object Tag" has entered the Trigger Bounds. If true, apply damage to the Self Actor
  (if (Actor|ActorHasTag OtherActor (Variables|Tag|GetObjectTag))
    (Game|Damage|ApplyDamage self 1e+01 0 0)
    (else
      (Development|PrintString "STATICAI: No Damage") ; I only expect this to run once.
    )))

(event Game|Damage|EventAnyDamage
  (params (Damage :type Float%20%28single-precision%29) (DamageType :type Damage%20Type%20Object%20Reference) (InstigatedBy :type Controller%20Object%20Reference) (DamageCauser :type Actor%20Object%20Reference))
  ;[0 1 0.2355] AI Health System
  (Variables|AIHealth|SetAIHealth (- (Variables|AIHealth|GetAIHealth) Damage))
  (if (<= (Variables|AIHealth|GetAIHealth) 0.0)
    (Utilities|FlowControl|DoOnce false
      (:Completed
        (Development|PrintString "STATICAI: AI Eliminated" true true "(R=1.000000,G=0.000000,B=0.000000,A=1.000000)")
        ;[1 0 0.1612] When Health Hits Zero, preform these functions
        (Physics|SetSimulatePhysics (Variables|Default|GetStaticMesh) true)
        (Audio|PlaySoundatLocation "/Engine/VREditor/Sounds/UI/Camera_Shutter.Camera_Shutter" (Transformation|GetActorLocation self) "0, 0, 0" 0.002 1.0 0.0 0 0 0 0) ; Need Appropriate SFX
        (Utilities|FlowControl|Delay 2.0)
        (Actor|DestroyActor)))
    (else
      (Development|PrintString (Utilities|String|ToString(Float) (Variables|AIHealth|GetAIHealth)) true true "(R=0.036493,G=1.000000,B=0.000000,A=1.000000)"))))

(fn ConstructionScript)

(event Custom|InstaKill
  ;[1 1 1] Instakill Obscicles
  (Game|Damage|ApplyDamage self 1e+02 0 0))