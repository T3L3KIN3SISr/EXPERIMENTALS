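; Dash power-up pickup that unlocks dashing for the first-person player character.
; Overlapping its box with that character sets CanPlayerDash, adds a particle system component using the camera's relative transform, and prints a debug message.
; It also plays the dash-enabled pulse animation on the player's UI widget, then destroys itself after a short delay.
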(event OnComponentBeginOverlap(Box)
  (params (OverlappedComponent :type Primitive%20Component%20Object%20Reference) (OtherActor :type Actor%20Object%20Reference) (OtherComp :type Primitive%20Component%20Object%20Reference) (OtherBodyIndex :type Integer) (bFromSweep :type Boolean) (SweepResult :type Hit%20Result%20Structure%20%28by%20ref%29))
  (bind _asbp_first_person_character (Utilities|Casting|CastToBP_FirstPersonCharacter OtherActor))
  (Development|PrintString "PLAYERDSH: Player can now Dash")
  (AddComponent|AddParticleSystemComponent _asbp_first_person_character false (Transformation|GetRelativeTransform (Variables|/Game/Blueprints/PlayerBlueprints/BP_FirstPersonCharacter.BP_FirstPersonCharacter_C|GetFirstPersonCamera _asbp_first_person_character)))
  (Variables|/Game/Blueprints/PlayerBlueprints/BP_FirstPersonCharacter.BP_FirstPersonCharacter_C|SetbCanPlayerDash? _asbp_first_person_character true)
  (Components|Animation|PlayAnimation (Variables|/Game/Blueprints/PlayerBlueprints/BP_FirstPersonCharacter.BP_FirstPersonCharacter_C|GetPlayer%20UI%20Reference _asbp_first_person_character) (Variables|/Game/UI/WB_PlayerUI.WB_PlayerUI_C|GetDashEnabledImagePulse (Variables|/Game/Blueprints/PlayerBlueprints/BP_FirstPersonCharacter.BP_FirstPersonCharacter_C|GetPlayer%20UI%20Reference _asbp_first_person_character)) 0.0
    (:then
      (Utilities|FlowControl|Delay 0.2)
      (Actor|DestroyActor))))

(fn ConstructionScript)