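; BP_Server_Controller is a capture-style server objective whose percentage rises near the player and falls near enemy AI.
; Two detection boxes check actor tags and run looping timers that increase or decrease the value.
; Reaching full locks out decreases and opens the referenced gate door once.
; The text render updates only while incrementing, and the spotlight switches red or green when the player or enemy leaves its box.
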(event OnComponentEndOverlap(PlayerDetectionBox)
  (params (OverlappedComponent :type Primitive%20Component%20Object%20Reference) (OtherActor :type Actor%20Object%20Reference) (OtherComp :type Primitive%20Component%20Object%20Reference) (OtherBodyIndex :type Integer))
  ;[0.09448 1 0] Stop Increasing Server Float when the Player has left the PlayerDetection Box
  (if (Actor|ActorHasTag OtherActor "Player")
    (Utilities|Time|ClearandInvalidateTimerbyHandle (Variables|Default|GetServerPlayerTimerHandle))
    (Development|PrintString "stopping server")
    (CallFunction|ChangeLightColour)))

(event OnComponentBeginOverlap(PlayerDetectionBox)
  (params (OverlappedComponent :type Primitive%20Component%20Object%20Reference) (OtherActor :type Actor%20Object%20Reference) (OtherComp :type Primitive%20Component%20Object%20Reference) (OtherBodyIndex :type Integer) (bFromSweep :type Boolean) (SweepResult :type Hit%20Result%20Structure%20%28by%20ref%29))
  ;[0.09448 1 0] Increase Server Float when Player is in the PlayerDetectionBox
  (if (Actor|ActorHasTag OtherActor "Player")
    (bind _returnvalue (Utilities|Time|SetTimerbyEvent (delegate Custom|ServerIncreaseFloat) 0.1 true))
    (Variables|Default|SetServerPlayerTimerHandle _returnvalue)))

(event OnComponentBeginOverlap(EnemyDetectionBox)
  (params (OverlappedComponent :type Primitive%20Component%20Object%20Reference) (OtherActor :type Actor%20Object%20Reference) (OtherComp :type Primitive%20Component%20Object%20Reference) (OtherBodyIndex :type Integer) (bFromSweep :type Boolean) (SweepResult :type Hit%20Result%20Structure%20%28by%20ref%29))
  ;[1 0 0] Decrease Server Float when an Enemy has entered the EnemyDetectionBox
  (if (Actor|ActorHasTag OtherActor "EnemyAI")
    (bind _returnvalue (Utilities|Time|SetTimerbyEvent (delegate Custom|ServerDecreaseFloat) 0.1 true))
    (Variables|Default|SetServerEnemyTimerHandle _returnvalue)))

(event OnComponentEndOverlap(EnemyDetectionBox)
  (params (OverlappedComponent :type Primitive%20Component%20Object%20Reference) (OtherActor :type Actor%20Object%20Reference) (OtherComp :type Primitive%20Component%20Object%20Reference) (OtherBodyIndex :type Integer))
  ;[1 0 0] Stop Decreasing Float when the EnemyAI has left the EnemyDetectionBox
  (if (Actor|ActorHasTag OtherActor "EnemyAI")
    (Utilities|Time|ClearandInvalidateTimerbyHandle (Variables|Default|GetServerEnemyTimerHandle))
    (Development|PrintString "stopping server")
    (CallFunction|ChangeLightColour)))

(event Custom|UpdateTextOnServer
  ;[1 1 1] Update the Text when the Server Percentage Value is being Incremented
  (Rendering|Components|TextRender|SetText (Variables|Default|GetTextRender) (Utilities|Text|ToText(Float) (Variables|Default|GetServerPercentageValue) "HalfToEven"))
  ;[1 1 1] Force Set Text Value to 100
  (if (== (Variables|Default|GetServerPercentageValue) 9e+01)
    (Rendering|Components|TextRender|SetText (Variables|Default|GetTextRender) (Variables|Default|GetValue))))

(event Custom|ServerIncreaseFloat
  ;[0.09448 1 0] Increase Server Float when Player is in the PlayerDetectionBox
  (|IncreaseFloatCalculation))

(event Custom|ChangeLightColour
  (bind _spotlight (Variables|Default|GetSpotLight))
  ;[1 1 1] Check if the Server is Completed. If so, set the Spotlight Colour to Green. If not, set the Spotlight Colour to Red.
  (if (Variables|Default|GetbIsServerCompleted?)
    (Rendering|Components|Light|SetLightColor _spotlight "(R=0.074322,G=1.000000,B=0.214139,A=1.000000)" true)
    (Development|PrintString "LIGHT: Green Completed")
    (else
      (Rendering|Components|Light|SetLightColor _spotlight "(R=0.375000,G=0.027344,B=0.027344,A=1.000000)" true)
      (Development|PrintString "LIGHT: RED Not Completed"))))

(event Custom|ServerDecreaseFloat
  ;[1 0 0] Decrease Server Float when an Enemy has entered the EnemyDetectionBox
  (|DecreaseFloatCalculation))

(event Custom|GateDoorOpen
  ;[1 1 1] Open a Gate Door when the Server is Completed
  (if (Variables|Default|GetbIsServerCompleted?)
    (Default|StartMovingDoor (Variables|Default|GetGateDoorReference))))

(fn ConstructionScript)