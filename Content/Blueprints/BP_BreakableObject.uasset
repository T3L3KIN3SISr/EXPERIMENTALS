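; BP_BreakableObject is a breakable prop that shatters and is removed when hit by an actor tagged "Projectile".
; A hit on its BoxCollision fires a one-time break that plays a sound, enables physics on the box and mesh, and applies a broken-glass overlay material.
; After a short delay the actor destroys itself, with debug prints tracking the process.
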(event OnComponentHit(BoxCollision)
  (params (HitComponent :type Primitive%20Component%20Object%20Reference) (OtherActor :type Actor%20Object%20Reference) (OtherComp :type Primitive%20Component%20Object%20Reference) (NormalImpulse :type Vector :default "0, 0, 0") (Hit :type Hit%20Result%20Structure%20%28by%20ref%29))
  (Utilities|IsValid OtherActor
    (:Is%20Valid
      (if (Actor|ActorHasTag OtherActor "Projectile")
        (Utilities|FlowControl|DoOnce false
          (:Completed
            (Development|PrintString "BREAKABLE : Object is being removed in 1 Second" true true "(R=1.000000,G=0.887261,B=0.000000,A=1.000000)")
            (Audio|PlaySoundatLocation "/Engine/VREditor/Sounds/UI/Enter_Play.Enter_Play" (Transformation|GetActorLocation) "0, 0, 0" 1.0 1.0 0.0 0 0 0 0) ; Insert Cracking Sound Here
            (Physics|SetSimulatePhysics (Variables|Default|GetBoxCollision) true) ; Let the Object fall with Gravity
            (Rendering|Material|SetOverlayMaterial (Variables|Default|GetStaticMesh) "/Game/Materials/M_Glass_Broken.M_Glass_Broken" :!class /Script/Engine.MeshComponent) ; MAKE THIS TEXTURE BROKEN lmao
            (Utilities|FlowControl|Delay 1.0)
            (Actor|DestroyActor)
            (Development|PrintString "BREAKABLE : Object is DESTROYED" true true "(R=1.000000,G=0.000000,B=0.018362,A=1.000000)")))))
    (:Is%20Not%20Valid
      (Development|PrintString "Projectile is Not Valid"))))

(fn ConstructionScript)