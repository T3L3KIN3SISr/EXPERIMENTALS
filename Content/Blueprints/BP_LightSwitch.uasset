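; BP_LightSwitch is an interactable wall switch that toggles five spotlights on and off.
; The Interaction event, called by the interaction system in FP_Blueprint, drives a FlipFlop that alternates between showing and hiding the spotlight components.
; Each toggle plays a sound at the switch mesh's location and prints a debug message.
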(event EventInteraction
  (bind _spotlight0 (Variables|Default|GetSpotlight0))
  (bind _sm_lightswitch (Variables|Default|GetSM_LightSwitch))
  (Utilities|FlowControl|FlipFlop ; Using Flip Flop for Switch
    (:A
      ;[0 1 0.1084] Light Switch On
      (Audio|PlaySoundatLocation 0 (Transformation|GetWorldLocation _sm_lightswitch) "0, 0, 0" 1.0 1.0 0.0 0 0 0 0) ; Place Sound Effect Here
      (Rendering|SetVisibility _spotlight0 true false)
      (Development|PrintString "LIGHTSW: Light Switch is on" true true "(R=0.000000,G=1.000000,B=0.003300,A=1.000000)"))
    (:B
      ;[1 0 0.0374] Light Switch Off
      (Audio|PlaySoundatLocation 0 (Transformation|GetWorldLocation _sm_lightswitch) "0, 0, 0" 1.0 1.0 0.0 0 0 0 0) ; Place Sound Effect Here
      (Rendering|SetVisibility _spotlight0 false false)
      (Development|PrintString "LIGHTSW: Light Switch is off" true true "(R=1.000000,G=0.000000,B=0.019485,A=1.000000)"))))

(fn ConstructionScript)