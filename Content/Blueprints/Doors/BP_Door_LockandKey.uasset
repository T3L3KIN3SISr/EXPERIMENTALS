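; Locked door actor that the player opens and closes through interaction once its key has been picked up.
; PickUpKey, INTRO_Flashlight and FallbackOpenDoor all set PlayerHasKey and recolour the linked lock indicator.
; Interaction uses a FlipFlop to play or reverse a timeline that lerps the door's yaw, with sound, or plays a denial sound without the key.
; A box collision toggles the interact widget for Player-tagged actors.
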(event OnComponentBeginOverlap(BoxCollision)
  (params (OverlappedComponent :type Primitive%20Component%20Object%20Reference) (OtherActor :type Actor%20Object%20Reference) (OtherComp :type Primitive%20Component%20Object%20Reference) (OtherBodyIndex :type Integer) (bFromSweep :type Boolean) (SweepResult :type Hit%20Result%20Structure%20%28by%20ref%29))
  ;[1 1 1] Interaction Widget Visibility
  ;;[1 0.989 0.1032] Check if the Player has entered the Box Collision
  (if (Actor|ActorHasTag OtherActor "Player")
    ;;[0.07099 0.07567 1] Set Visibility of Widget
    (Rendering|SetVisibility (Variables|Default|GetInteractWidget) true false)))

(event OnComponentEndOverlap(BoxCollision)
  (params (OverlappedComponent :type Primitive%20Component%20Object%20Reference) (OtherActor :type Actor%20Object%20Reference) (OtherComp :type Primitive%20Component%20Object%20Reference) (OtherBodyIndex :type Integer))
  ;[1 1 1] Interaction Widget Visibility
  ;;[1 0.989 0.1032] Check if the Player has entered the Box Collision
  (if (Actor|ActorHasTag OtherActor "Player")
    ;;[0.07099 0.07567 1] Set Visibility of Widget
    (Rendering|SetVisibility (Variables|Default|GetInteractWidget) false false)))

(event Custom|FallbackOpenDoor
  ;[1 0 0.1041] Boolean Check from BP_CubeKey (ON PICK UP)
  (Variables|Default|SetbPlayerHasKey true)
  (Default|ChangeColour (Variables|Default|GetDoorLockIndicatorReference)))

(event Custom|INTRO_Flashlight
  ;[1 0 0.1041] Boolean Check from BP_CubeKey (ON PICK UP)
  (Variables|Default|SetbPlayerHasKey true)
  (Default|ChangeColour (Variables|Default|GetDoorLockIndicatorReference)))

(event EventInteraction
  (bind _self self)
  (bind _returnvalue (Transformation|GetActorLocation _self))
  ;[1 0.1227 0.7455] Door Open and Close - Event Interaction - Supported by Matt Aspland - https://www.youtube.com/watch?v=Bcle9sSS4Oo
  (if (Variables|Default|GetbPlayerHasKey) ; Check if the Player has picked up the Key
    (Utilities|FlowControl|FlipFlop ; A is Open. B is Close
      (:A
        (Audio|PlaySoundatLocation "/Game/Audio/SW_sci-fi-door-open-47994.SW_sci-fi-door-open-47994" _returnvalue "0, 0, 0" 1.0 1.0 0.0 0 0 0 0)
        (bind _doortrackalpha (Timeline|DoorTimeline Play)
          (:Update
            (Transformation|SetRelativeRotation (Variables|Default|GetSM_Door) (Math|Rotator|MakeRotator 0.0 0.0 (Math|Float|Lerp 0.0 1.1e+02 _doortrackalpha)) false false)
            (Utilities|FlowControl|DoOnce false ; Preventing Multiple Prints of following string
              (:Completed
                (Development|PrintString "DOORLOCK: Player has appropriate key. Opening Door!" true true "(R=0.000000,G=1.000000,B=0.111239,A=1.000000)") ; This would usually print out numerous times. Check DO ONCE
              )))))
      (:B
        (Audio|PlaySoundatLocation "/Game/Audio/SW_sci-fi-door-open-47994.SW_sci-fi-door-open-47994" _returnvalue "0, 0, 0" 1.0 1.0 0.0 0 0 0 0)
        (Timeline|DoorTimeline Reverse)))
    (else
      (Development|PrintString "DOORLOCK: You do not have the Dedicated Key for this Door!" true true "(R=1.000000,G=0.036710,B=0.000000,A=1.000000)")
      (Audio|PlaySoundatLocation "/Engine/EditorSounds/Notifications/CompileFailed.CompileFailed" (Transformation|GetActorLocation self) "0, 0, 0" 1.0 1.0 0.0 0 0 0 0))))

(event EventPickUpKey
  ;[1 0 0.1041] Boolean Check from BP_CubeKey (ON PICK UP)
  (Variables|Default|SetbPlayerHasKey true)
  (Default|ChangeColour (Variables|Default|GetDoorLockIndicatorReference)))

(fn ConstructionScript)