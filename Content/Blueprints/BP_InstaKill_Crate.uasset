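; BP_InstaKill_Crate is a physics crate that triggers an instant kill on an AI.
; On BeginPlay, both its StaticMesh and Box simulate physics.
; When the Box begins an overlap and the other actor has overlapping actors matching a class filter, it calls InstaKill on the stored AIReference rather than on the overlapping actor.
; Debug prints report the trigger and an invalid reference.
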(event OnComponentBeginOverlap(Box)
  (params (OverlappedComponent :type Primitive%20Component%20Object%20Reference) (OtherActor :type Actor%20Object%20Reference) (OtherComp :type Primitive%20Component%20Object%20Reference) (OtherBodyIndex :type Integer) (bFromSweep :type Boolean) (SweepResult :type Hit%20Result%20Structure%20%28by%20ref%29))
  (bind _ai_reference (Variables|Default|GetAI%20Reference))
  (if (Math|Conversions|ToBoolean(Integer) (Utilities|Array|Length (Collision|GetOverlappingActors OtherActor (Variables|Default|GetClass%20Filter) :!class /Script/Engine.Actor)))
    (Development|PrintString "INSTAKILL")
    (Utilities|IsValid _ai_reference
      (:Is%20Valid
        (Default|InstaKill _ai_reference))
      (:Is%20Not%20Valid
        (Development|PrintString "NotValid")))))

(event EventBeginPlay
  (Physics|SetSimulatePhysics (Variables|Default|GetStaticMesh) true))

(fn ConstructionScript)