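; BP_DoorAuto is a door that swings open automatically when the first-person character enters its box trigger and closes when they leave.
; Overlap events set IsNearDoor and call DoorOpen or DoorClose, which play or reverse a timeline that lerps the door mesh's yaw.
; DoN caps open calls at five, but un-reset DoOnce nodes let opening and closing each run only once.
; Debug prints trace the entry overlap.
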(event OnComponentBeginOverlap(BoxCollisionTrigger)
  (params (OverlappedComponent :type Primitive%20Component%20Object%20Reference) (OtherActor :type Actor%20Object%20Reference) (OtherComp :type Primitive%20Component%20Object%20Reference) (OtherBodyIndex :type Integer) (bFromSweep :type Boolean) (SweepResult :type Hit%20Result%20Structure%20%28by%20ref%29))
  (bind _asbp_first_person_character (Utilities|Casting|CastToBP_FirstPersonCharacter OtherActor))
  (Development|PrintString "Casting")
  (Utilities|IsValid _asbp_first_person_character
    (:Is%20Valid
      (Development|PrintString "is Valid")
      (Variables|Default|SetIsNearDoor true)
      (bind _counter (Utilities|FlowControl|DoN 5)
        (:Exit
          (CallFunction|DoorOpen)
          (Development|PrintString (Utilities|String|ToString(Integer) _counter)))))
    (:Is%20Not%20Valid
      (Development|PrintString "Not Valid")
      (Variables|Default|SetIsNearDoor false))))

(event OnComponentEndOverlap(BoxCollisionTrigger)
  (params (OverlappedComponent :type Primitive%20Component%20Object%20Reference) (OtherActor :type Actor%20Object%20Reference) (OtherComp :type Primitive%20Component%20Object%20Reference) (OtherBodyIndex :type Integer))
  (bind _asbp_first_person_character (Utilities|Casting|CastToBP_FirstPersonCharacter OtherActor))
  (Utilities|IsValid _asbp_first_person_character
    (:Is%20Valid
      (Variables|Default|SetIsNearDoor false)
      (CallFunction|DoorClose))))

(event Custom|DoorOpen
  (if (Variables|Default|GetIsNearDoor)
    (Utilities|FlowControl|DoOnce false
      (:Completed
        (bind _doormovementalpha (Timeline|DoorMovementTimeline PlayFromStart)
          (:Update
            (Transformation|SetRelativeRotation (Variables|Default|GetSM_Door) (Math|Rotator|MakeRotator 0.0 0.0 (.z (Math|Vector|Lerp(Vector) (Variables|DoorSetup|GetDoorStart) (Variables|DoorSetup|GetDoorEnd) _doormovementalpha))) false false)))))))

(event Custom|DoorClose
  (Utilities|FlowControl|DoOnce false
    (:Completed
      (bind _doormovementalpha (Timeline|DoorMovementTimeline Reverse)
        (:Update
          (Transformation|SetRelativeRotation (Variables|Default|GetSM_Door) (Math|Rotator|MakeRotator 0.0 0.0 (.z (Math|Vector|Lerp(Vector) (Variables|DoorSetup|GetDoorStart) (Variables|DoorSetup|GetDoorEnd) _doormovementalpha))) false false))))))

(fn ConstructionScript)