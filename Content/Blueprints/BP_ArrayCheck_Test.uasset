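; BP_ArrayCheck_Test is a test target that destroys itself when a Projectile-tagged actor hits its Box, spawning a key cube at a set remaining count.
; After DestroyActor, a custom event counts actors of its class with GetAllActorsOfClass.
; If exactly three remain and HasCubeSpawned is false, it temporarily spawns BP_CubeKey at the player's transform.
; Other counts print an "already spawned" message, even if none has spawned.
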(event OnComponentHit(Box)
  (params (HitComponent :type Primitive%20Component%20Object%20Reference) (OtherActor :type Actor%20Object%20Reference) (OtherComp :type Primitive%20Component%20Object%20Reference) (NormalImpulse :type Vector :default "0, 0, 0") (Hit :type Hit%20Result%20Structure%20%28by%20ref%29))
  ;[1 1 1] Check for "Projectile" Tag and Call Custom Event
  (if (Actor|ActorHasTag OtherActor "Projectile")
    (Physics|SetSimulatePhysics (Variables|Default|GetSkeletalMesh) true)
    (Actor|DestroyActor)
    (CallFunction|CustomEvent)))

(event Custom|CustomEvent
  (Utilities|FlowControl|Sequence
    (:then_0
      ;[1 1 1] Constant Check Array and Set Variable
      (bind _outactors (Actor|GetAllActorsOfClass "BP_ArrayCheck_Test_C"))
      (Variables|Default|SetActorsLeft (Utilities|Array|Length _outactors)))
    (:then_1
      ;[1 1 1] Dual Boolean Condition Check
      (if (not (Variables|Default|GetbHasCubeSpawned?))
        (if (== (Variables|Default|GetActorsLeft) 3)
          ;[1 1 1] Spawn Cube in front of Player (Temporary)
          (bind _asbp_first_person_character (Utilities|Casting|CastToBP_FirstPersonCharacter (Game|Player|GetPlayerPawn 0)))
          ;[1 1 1] Spawn Cube Key and Activate Spawned Cube Boolean
          (Game|SpawnActorfromClass "/Game/Blueprints/Doors/BP_CubeKey.BP_CubeKey_C" (Transformation|GetActorTransform _asbp_first_person_character) "Undefined" "MultiplyWithRoot" 0 0 0)
          (Variables|Default|SetbHasCubeSpawned? true)
          (else
            (Development|PrintString "ARRAYCHK: Cube has already spawned! Not Spawning another.")))))))

(fn ConstructionScript)