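; Windmill Blueprint, partly marked as tutorial, with blades that spin and can be destroyed by projectiles.
; Key 1 plays a timeline that drives blade pitch from a multiplied rotation track.
; A "Projectile"-tagged hit on the box spawns fire, then after a delay adds an explosion and collapse sound, enables blade physics and stops the timeline.
; A separate graph sets WindmillSpeed on both press and release of N.
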(event OnComponentHit(Box)
  (params (HitComponent :type Primitive%20Component%20Object%20Reference) (OtherActor :type Actor%20Object%20Reference) (OtherComp :type Primitive%20Component%20Object%20Reference) (NormalImpulse :type Vector :default "0, 0, 0") (Hit :type Hit%20Result%20Structure%20%28by%20ref%29))
  ;[1 0.8768 0.7948] Check if the "Projectile" Tag has hit the Box Collision
  (if (Actor|ActorHasTag OtherActor "Projectile")
    ;[1 0.1458 0.8922] Handling Particles using OTF Variables \ Setting Physics and Delays
    (bind _output_get (Variables|Default|SetFireTransform (Math|Transform|MakeTransform "0, 0, 0" "0, 0, 0" "5.000000,5.000000,5.000000")))
    (AddComponent|AddParticleSystemComponent false _output_get) ; Start the "Fire" Particles
    (Utilities|FlowControl|Delay 4.0) ; Let the Fire BURNN! for 4 Seconds
    (bind _output_get_2 (Variables|Default|SetBladeExplosionTransform (Math|Transform|MakeTransform "0.000000,110.000000,330.000000" "0, 0, 0" "1.000000,1.000000,1.000000")))
    (AddComponent|AddParticleSystemComponent false _output_get_2) ; Start the "Explosion" Particles
    (Audio|PlaySoundatLocation "/Game/Misc/StarterContent/Audio/Collapse02.Collapse02" (Transformation|GetActorLocation) "0, 0, 0" 1.0 1.0 0.0 0 0 0 0)
    (Physics|SetSimulatePhysics (Variables|Default|GetSM_Windmill_Blades) true) ; Allow Physics to be turned on
    ;[1 1 1] Play Animation on Windmill Blades (Tutorial)
    (bind _bladerotation (Timeline|WindmillTimeline Stop)
      (:Update
        (Transformation|SetRelativeRotation (Variables|Default|GetSM_Windmill_Blades) (Math|Rotator|MakeRotator 0.0 (* _bladerotation (|MultiplyFloat)) 0.0) false false)))))

(event Input|KeyboardEvents|1
  (params (Key :type Key%20Structure))
  ;[1 1 1] Play Animation on Windmill Blades (Tutorial)
  (:Pressed
    (bind _bladerotation (Timeline|WindmillTimeline Play)
      (:Update
        (Transformation|SetRelativeRotation (Variables|Default|GetSM_Windmill_Blades) (Math|Rotator|MakeRotator 0.0 (* _bladerotation (|MultiplyFloat)) 0.0) false false)))))

(fn ConstructionScript)

(event Input|KeyboardEvents|N
  (params (Key :type Key%20Structure))
  (:Pressed
    (bind _output_get (Variables|Default|SetWindmillSpeed 5.0 :!label _label))
    (bind _output_get_2 (Variables|Default|SetWindmillSpeed (* _output_get 2e+01))))
  (:Released
    (goto _label)))