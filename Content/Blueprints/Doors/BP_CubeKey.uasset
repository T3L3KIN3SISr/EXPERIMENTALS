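; BP_CubeKey is a pickup key that unlocks a linked lock-and-key door.
; Actor overlap toggles an outline overlay material and an interact widget as a proximity cue.
; Its Interaction event sends PickUpKeyMessage to the per-instance door reference, plays a sound, prints a debug message and destroys the key.
; Physics simulation on the mesh and interaction box starts after a short BeginPlay delay, keeping the key suspended until then.
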(event EventBeginPlay
  ;[1 1 1] Sustain Object in Air for Specific Delay and then Apply Physics
  (Utilities|FlowControl|Delay 5.0)
  (Physics|SetSimulatePhysics (Variables|Default|GetInteractionBox) true))

(event Collision|EventActorBeginOverlap
  (params (OtherActor :type Actor%20Object%20Reference))
  ;[1 1 1] Add Material Overlay when Player is near
  ;;[0.2075 1 0] On
  (Rendering|Material|SetOverlayMaterial (Variables|Default|GetStaticMesh) "/Game/Materials/M_OutlineInteract_Inst.M_OutlineInteract_Inst" :!class /Script/Engine.MeshComponent)
  ;;[0.03709 0.05768 1] Set Visibility of Interact Widget
  (Rendering|SetVisibility (Variables|Default|GetWidget) true false))

(event EventInteraction
  ;[1 1 1] Event Interaction for Boolean Check in BP_Door_LockandKey
  (Class|BPIDoor|PickUpKey(Message) (Variables|Default|GetDoorBlueprint))
  (Audio|PlaySoundatLocation "/Game/Audio/SW_item-equip-6904.SW_item-equip-6904" (Transformation|GetActorLocation self) "0, 0, 0" 0.5 1.0 0.0 0 0 0 0)
  (Actor|DestroyActor)
  (Development|PrintString "DOORKEY: A Key for a LOCKDOOR has been picked up!"))

(event Collision|EventActorEndOverlap
  (params (OtherActor :type Actor%20Object%20Reference))
  ;[1 1 1] Add Material Overlay when Player is near
  ;;[1 0 0] Off
  (Rendering|Material|SetOverlayMaterial (Variables|Default|GetStaticMesh) 0 :!class /Script/Engine.MeshComponent)
  ;;[0.03709 0.05768 1] Set Visibility of Interact Widget
  (Rendering|SetVisibility (Variables|Default|GetWidget) false false))

(fn ConstructionScript)