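; Poison projectile, kept with the AI projectile assets, that poisons the player on contact.
; When its Sphere overlaps an actor tagged Player, it casts to BP_FirstPersonCharacter, calls PoisonPlayer and sets IsPlayerPoisoned.
; It then destroys itself after a short delay, whose length depends on a self-validity check.
; This graph ignores other overlaps and contains no movement logic.
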(event OnComponentBeginOverlap(Sphere)
  (params (OverlappedComponent :type Primitive%20Component%20Object%20Reference) (OtherActor :type Actor%20Object%20Reference) (OtherComp :type Primitive%20Component%20Object%20Reference) (OtherBodyIndex :type Integer) (bFromSweep :type Boolean) (SweepResult :type Hit%20Result%20Structure%20%28by%20ref%29))
  ;[1 0.8671 0] Check if the Projectile has Overlapped \ Hit the Player
  (if (Actor|ActorHasTag OtherActor "Player")
    ;[0 1 0.03429] Call the Poison Player Event in FirstPerson Character
    (bind _asbp_first_person_character (Utilities|Casting|CastToBP_FirstPersonCharacter OtherActor)) ; Get Active Instance
    (Default|PoisonPlayer _asbp_first_person_character)
    (Variables|/Game/Blueprints/PlayerBlueprints/BP_FirstPersonCharacter.BP_FirstPersonCharacter_C|SetbIsPlayerPoisoned? _asbp_first_person_character true) ; Set Boolean to True (might not be needed..?)
    ;[0.7293 0.319 1] Check for Object Validity and then Destroy Actor (Prevent Garbage Error)
    (Utilities|IsValid self
      (:Is%20Valid
        (Utilities|FlowControl|Delay 2.0)
        (Actor|DestroyActor))
      (:Is%20Not%20Valid
        (Utilities|FlowControl|Delay 3.0)
        (Actor|DestroyActor)))))

(fn ConstructionScript)