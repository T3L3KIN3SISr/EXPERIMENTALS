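; BP_Platform_Delay is a fragile glass platform that cracks, then collapses after a player steps on it.
; Box overlap by a Player-tagged actor starts delayed stages: break sound, cracked overlay material, collapse sound and physics simulation.
; After falling, it disables physics and sets the actor transform to the mesh's relative transform saved at BeginPlay.
; DoOnce gates are never reset and the overlay is never cleared.
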(event OnComponentBeginOverlap(Box)
  (params (OverlappedComponent :type Primitive%20Component%20Object%20Reference) (OtherActor :type Actor%20Object%20Reference) (OtherComp :type Primitive%20Component%20Object%20Reference) (OtherBodyIndex :type Integer) (bFromSweep :type Boolean) (SweepResult :type Hit%20Result%20Structure%20%28by%20ref%29))
  (Utilities|FlowControl|DoOnce false
    (:Completed
      (bind _output_get (Variables|Default|SetbIsPlayerOnFragilePlatform? (Actor|ActorHasTag OtherActor "Player")))
      (if _output_get
        (Audio|PlaySoundatLocation "/Game/Audio/SW_glass-break-3-102271.SW_glass-break-3-102271" (Transformation|GetActorLocation self) "0, 0, 0" 1.0 1.0 0.0 0 0 0 0)
        (Utilities|FlowControl|Delay 1.0)
        (Rendering|Material|SetOverlayMaterial (Variables|Default|GetStaticMesh) "/Game/Materials/M_Glass_Broken.M_Glass_Broken" :!class /Script/Engine.MeshComponent)
        (Development|PrintString "PLATFORMDL: Platform is about to BREAK!")
        (Utilities|FlowControl|Delay 6.0)
        (Audio|PlaySoundatLocation "/Game/Misc/StarterContent/Audio/Collapse01.Collapse01" (Transformation|GetActorLocation self) "0, 0, 0" 1.0 1.0 0.0 0 0 0 0)
        (Physics|SetSimulatePhysics (Variables|Default|GetBox) true)
        (Development|PrintString "PLATFORMDL: Platform has fallen! Resetting Platform in 5 Seconds")
        (Utilities|FlowControl|Delay 5.0)
        (Physics|SetSimulatePhysics (Variables|Default|GetBox) false)
        (CallFunction|ResetPlatform)))))

(event OnComponentEndOverlap(Box)
  (params (OverlappedComponent :type Primitive%20Component%20Object%20Reference) (OtherActor :type Actor%20Object%20Reference) (OtherComp :type Primitive%20Component%20Object%20Reference) (OtherBodyIndex :type Integer))
  (Utilities|FlowControl|DoOnce false
    (:Completed
      (if (Actor|ActorHasTag OtherActor "Player")
        (Variables|Default|SetbIsPlayerOnFragilePlatform? false)
        (else
          (Variables|Default|SetbIsPlayerOnFragilePlatform? true))))))

(event Custom|ResetPlatform
  (Transformation|SetActorTransform (Variables|Default|GetOriginalPlatformTransform))
  (Development|PrintString "Hello"))

(event EventBeginPlay
  (Variables|Default|SetOriginalPlatformTransform (Transformation|GetRelativeTransform (Variables|Default|GetStaticMesh))))

(fn ConstructionScript)