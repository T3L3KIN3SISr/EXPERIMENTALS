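; BP_GateTrigger is a trigger that opens or moves a gate door when a set number of objects occupy its box.
; On each begin overlap, it counts overlapping actors of an instance-selectable class and shows the count on a text render.
; When the count exactly equals the per-instance target, it calls StartMovingDoor on the referenced gate door; end overlaps are not handled.
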(event OnComponentBeginOverlap(TriggerBox)
  (params (OverlappedComponent :type Primitive%20Component%20Object%20Reference) (OtherActor :type Actor%20Object%20Reference) (OtherComp :type Primitive%20Component%20Object%20Reference) (OtherBodyIndex :type Integer) (bFromSweep :type Boolean) (SweepResult :type Hit%20Result%20Structure%20%28by%20ref%29))
  ;[1 0.7219 0] Check for how many Objects are in the BoxCollision Component.
  ;[0.5877 0.307 1] Check the Array Value and see if its equal to the "Is Equal to?" Inst. Variable
  (bind _output_get (Variables|Default|SetArrayLength (Utilities|Array|Length (Collision|GetOverlappingActors (Variables|Default|GetTriggerBox) (Variables|Settings|GetWhich%20Object%20should%20be%20Checked?) :!class /Script/Engine.PrimitiveComponent))))
  ;[1 0.3521 0.7462] Print Text on the Text Render
  (Rendering|Components|TextRender|SetText (Variables|Default|GetTextRender) (Utilities|Text|ToText(Integer) (Variables|Default|GetArrayLength)))
  ;[1 0.3552 0.3552] Check the Condition of the Boolean.
  (if (== _output_get (Variables|Settings|GetisEqualTo?))
    (Default|StartMovingDoor (Variables|Settings|GetGateDoorObject))))

(fn ConstructionScript)