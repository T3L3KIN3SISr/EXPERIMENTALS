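; BP_Door_LockIndicator is a door lock indicator that shows whether its referenced door is unlocked or locked.
; Its ChangeColour event reads PlayerHasKey from DoorReference and swaps the Cube's material between the open and locked lock materials.
; Both branches also play a sound at the actor's location and print the lock state to the screen.
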(event Custom|ChangeColour
  (bind _self self)
  (bind _cube (Variables|Default|GetCube))
  (bind _returnvalue (Transformation|GetActorLocation _self))
  (if (Variables|/Game/Blueprints/Doors/BP_Door_LockandKey.BP_Door_LockAndKey_C|GetbPlayerHasKey (Variables|Default|GetDoorReference))
    (Audio|PlaySoundatLocation 0 _returnvalue "0, 0, 0" 1.0 1.0 0.0 0 0 0 0)
    (Rendering|Material|SetMaterial _cube 0 "/Game/Materials/M_DoorLock_Open.M_DoorLock_Open")
    (Development|PrintString "Door is Unlocked!")
    (else
      (Audio|PlaySoundatLocation 0 _returnvalue "0, 0, 0" 1.0 1.0 0.0 0 0 0 0)
      (Rendering|Material|SetMaterial _cube 0 "/Game/Materials/M_DoorLock_Locked.M_DoorLock_Locked")
      (Development|PrintString "Door is Locked!"))))

(fn ConstructionScript)