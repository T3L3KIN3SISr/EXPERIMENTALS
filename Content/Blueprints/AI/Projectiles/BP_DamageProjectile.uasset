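; BP_DamageProjectile is an AI projectile actor that damages the player when its Sphere overlaps them.
; The overlap checks for the Player tag, casts to BP_FirstPersonCharacter and calls DamagePlayer.
; A DoOnce limits damage to one hit per projectile instance.
; After the hit, the projectile destroys itself following a short delay, whose length depends on an IsValid check on itself.
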(event OnComponentBeginOverlap(Sphere)
  (params (OverlappedComponent :type Primitive%20Component%20Object%20Reference) (OtherActor :type Actor%20Object%20Reference) (OtherComp :type Primitive%20Component%20Object%20Reference) (OtherBodyIndex :type Integer) (bFromSweep :type Boolean) (SweepResult :type Hit%20Result%20Structure%20%28by%20ref%29))
  ;[1 0.7567 0] Check if the Projectile has hit the Player
  (if (Actor|ActorHasTag OtherActor "Player")
    (bind _asbp_first_person_character (Utilities|Casting|CastToBP_FirstPersonCharacter OtherActor)) ; Get Active Instance
    ;[1 0 0.06996] Only Damage the Player Once per Object Instance
    (Utilities|FlowControl|DoOnce false
      (:Completed
        (Default|DamagePlayer _asbp_first_person_character)
        ;[0.7293 0.319 1] Check for Object Validity and then Destroy Actor (Prevent Garbage Error)
        (Utilities|IsValid self
          (:Is%20Valid
            (Utilities|FlowControl|Delay 2.0)
            (Actor|DestroyActor))
          (:Is%20Not%20Valid
            (Utilities|FlowControl|Delay 3.0)
            (Actor|DestroyActor)))))))

(fn ConstructionScript)