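; Interactable medical kit that heals the first-person player once, by an instance-editable amount, when health is below full.
; Interaction adds the health; if the result clears the low-health threshold, it stops the low-health effect, caps health at 100, plays a sound and destroys the kit after a brief delay.
; Actor overlap toggles an outline overlay material and the interaction prompt widget.
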(event EventInteraction
  (bind _asbp_first_person_character (Utilities|Casting|CastToBP_FirstPersonCharacter (Game|Player|GetPlayerPawn 0))) ; Casting due to BP always being active in Instance. No need for VarReference
  (Variables|Default|SetPlayerReference _asbp_first_person_character)
  (if (< (Variables|/Game/Blueprints/PlayerBlueprints/BP_FirstPersonCharacter.BP_FirstPersonCharacter_C|GetPlayerHealth (Variables|Default|GetPlayerReference)) 1e+02)
    ;[0.427 1 0.2785] If Player Health is less than 100, add "Player Health Replenish Value" to Player Health. (Instance Editable Variable)
    (Utilities|FlowControl|DoOnce false
      (:Completed
        (bind _output_get (Variables|/Game/Blueprints/PlayerBlueprints/BP_FirstPersonCharacter.BP_FirstPersonCharacter_C|SetPlayerHealth (Variables|Default|GetPlayerReference) (+ (Variables|/Game/Blueprints/PlayerBlueprints/BP_FirstPersonCharacter.BP_FirstPersonCharacter_C|GetPlayerHealth (Variables|Default|GetPlayerReference)) (Variables|Replenish|GetPlayerHealthReplenishValue))))
        (Development|PrintString (Utilities|String|ToString(Float) _output_get))
        (if (> (Variables|/Game/Blueprints/PlayerBlueprints/BP_FirstPersonCharacter.BP_FirstPersonCharacter_C|GetPlayerHealth (Variables|Default|GetPlayerReference)) 35.0)
          (Default|StopLowHealthFunction (Variables|Default|GetPlayerReference))
          ;[1 0.2893 0.2056] If the Player Health Value is Greater than 100. Force Set the Value back to 100
          (if (> (Variables|/Game/Blueprints/PlayerBlueprints/BP_FirstPersonCharacter.BP_FirstPersonCharacter_C|GetPlayerHealth (Variables|Default|GetPlayerReference)) 1e+02)
            (bind _output_get_2 (Variables|/Game/Blueprints/PlayerBlueprints/BP_FirstPersonCharacter.BP_FirstPersonCharacter_C|SetPlayerHealth (Variables|Default|GetPlayerReference) 1e+02)) ; Force Set Float Value
            (Development|PrintString (Utilities|String|ToString(Float) _output_get_2)))
          ;[1 0.4962 0.2319] Play Sound and Destroy Actor
          (Audio|PlaySoundatLocation "/Engine/EngineSounds/1kSineTonePing.1kSineTonePing" (Transformation|GetActorLocation) "0, 0, 0" 1.0 1.0 0.0 0 0 0 0)
          (Development|PrintString "MEDICAL: Player is being healed." true true "(R=0.119021,G=1.000000,B=0.000000,A=1.000000)")
          (Utilities|FlowControl|Delay 0.2) ; An Attempt to prevent Validity Errors.
          (Actor|DestroyActor))))))

(event Collision|EventActorBeginOverlap
  (params (OtherActor :type Actor%20Object%20Reference))
  ;[1 1 1] Add Material Overlay when Player is near
  ;;[0.2075 1 0] On
  (Rendering|Material|SetOverlayMaterial (Variables|Default|GetHealthObject) "/Game/Materials/M_OutlineInteract_Inst.M_OutlineInteract_Inst" :!class /Script/Engine.MeshComponent)
  ;;[0.03709 0.05768 1] Set Visibility of Interact Widget
  (Rendering|SetVisibility (Variables|Default|GetWidget) true false))

(event Collision|EventActorEndOverlap
  (params (OtherActor :type Actor%20Object%20Reference))
  ;[1 1 1] Add Material Overlay when Player is near
  ;;[1 0 0] Off
  (Rendering|Material|SetOverlayMaterial (Variables|Default|GetHealthObject) 0 :!class /Script/Engine.MeshComponent)
  ;;[0.03709 0.05768 1] Set Visibility of Interact Widget
  (Rendering|SetVisibility (Variables|Default|GetWidget) false false))

(fn ConstructionScript)